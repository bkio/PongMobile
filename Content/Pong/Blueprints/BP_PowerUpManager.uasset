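; BP_PowerUpManager displays on-screen announcements when a power-up activates in the Pong game.
; On BeginPlay it creates the power-up widget for the first player and adds it to the viewport.
; PowerUpActivated switches on the power-up type to set the message, naming player or opponent for non-ball effects.
; A retriggerable delay clears the text shortly afterward, restarting whenever another activation arrives.
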(event EventBeginPlay
  (bind _returnvalue (UserInterface|CreateWidget "/Game/Pong/Widgets/PowerUpWidget.PowerUpWidget_C" (Game|GetPlayerController 0)))
  (bind _output_get (Variables|Default|SetPowerUpWidget _returnvalue))
  (UserInterface|Viewport|AddtoViewport _output_get 0))

(event EventPowerUpActivated
  (params (PowerUpType :type EPowerUpType%20Enum) (IsActivatedForPlayer :type Boolean))
  (bind _returnvalue (Utilities|String|SelectString "you!" "opponent!" IsActivatedForPlayer))
  (bind _powerupwidget (Variables|Default|GetPowerUpWidget))
  (bind _returnvalue_2 (Utilities|String|Append " for " _returnvalue))
  (bind _activatedpowerup_text (Variables|/Game/Pong/Widgets/PowerUpWidget.PowerUpWidget_C|GetActivatedPowerUp_Text _powerupwidget))
  (switch Utilities|FlowControl|Switch|SwitchonEPowerUpType PowerUpType
    (:SpeedBoost
      (Rendering|Components|TextRender|SetText _activatedpowerup_text (Utilities|Text|ToText(String) (Utilities|String|Append "Speed boost" _returnvalue_2))))
    (:StickyPaddle
      (Rendering|Components|TextRender|SetText _activatedpowerup_text (Utilities|Text|ToText(String) (Utilities|String|Append "Sticky paddle" _returnvalue_2))))
    (:InvisibleBall
      (Rendering|Components|TextRender|SetText _activatedpowerup_text "Invisible Ball!"))
    (:ReverseKeys
      (Rendering|Components|TextRender|SetText _activatedpowerup_text (Utilities|Text|ToText(String) (Utilities|String|Append "Controls are reversed" _returnvalue_2))))
    (:ShrinkBall
      (Rendering|Components|TextRender|SetText _activatedpowerup_text "Ball is shrunken!")))
  (Utilities|FlowControl|RetriggerableDelay 1.0)
  (Rendering|Components|TextRender|SetText (Variables|/Game/Pong/Widgets/PowerUpWidget.PowerUpWidget_C|GetActivatedPowerUp_Text (Variables|Default|GetPowerUpWidget)) ""))

(fn ConstructionScript)