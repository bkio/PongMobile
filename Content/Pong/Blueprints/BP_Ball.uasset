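; BP_Ball is the Pong ball Blueprint, providing animated visibility fades and size changes.
; SetBallRenderVisibility and ChangeBallSize each reset a counter and open a Gate on Tick, which runs a linear ease until done.
; Visibility drives the BallVisibility scalar in the PongMaterialParameters collection.
; Sizing moves between default and half collision radius, scaling the mesh and offsetting its Z to match, using defaults cached on BeginPlay.
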(event EventSetBallRenderVisibility
  (params (NewVisibility :type Boolean))
  (bind _static_zero (Variables|StaticValues|GetStatic_Zero))
  (bind _static_one (Variables|StaticValues|GetStatic_One))
  (Variables|Visibility|SetNewRenderVisibility NewVisibility)
  (Variables|Visibility|SetVisibilityChange_Counter 0.0)
  (Utilities|FlowControl|Gate true) ; enters at Open
)

(event EventTick
  (params (DeltaSeconds :type Float%20%28single-precision%29))
  (bind _returnvalue (* DeltaSeconds 1.25))
  (bind _newshrinkstatus (Variables|Size|GetNewShrinkStatus))
  (bind _defaultsphereradius (Variables|Defaults|GetDefaultSphereRadius))
  (bind _staticmesh (Variables|Default|GetStaticMesh))
  (bind _defaultsphereradius_2 (Variables|Defaults|GetDefaultSphereRadius))
  (bind _static_zero (Variables|StaticValues|GetStatic_Zero))
  (bind _static_one (Variables|StaticValues|GetStatic_One))
  (bind _newrendervisibility (Variables|Visibility|GetNewRenderVisibility))
  (bind _defaultrelativemeshlocation (Variables|Defaults|GetDefaultRelativeMeshLocation))
  (bind _returnvalue_2 (/ _defaultsphereradius 2.0))
  (bind (_x _y _z) (Math|Vector|BreakVector _defaultrelativemeshlocation))
  (Utilities|FlowControl|Sequence
    (:then_0
      (Utilities|FlowControl|Gate true :!label _label
        (:Exit
          (bind _output_get (Variables|Visibility|SetVisibilityChange_Counter (+ (Variables|Visibility|GetVisibilityChange_Counter) _returnvalue)))
          (Rendering|Material|SetScalarParameterValue "/Game/Pong/Materials/PongMaterialParameters.PongMaterialParameters" "BallVisibility" (Math|Interpolation|Ease "Linear" (Math|Float|Clamp(Float) _output_get) (Math|Float|SelectFloat _static_zero _static_one _newrendervisibility) (Math|Float|SelectFloat _static_one _static_zero _newrendervisibility)) :!class /Script/Engine.KismetMaterialLibrary)
          (if (>= (+ (Variables|Visibility|GetVisibilityChange_Counter) _returnvalue) 1.0)
            (goto _label Close)))))
    (:then_1
      (Utilities|FlowControl|Gate true :!label _label_2
        (:Exit
          (bind _output_get_2 (Variables|Size|SetSizeChange_Counter (+ (Variables|Size|GetSizeChange_Counter) _returnvalue)))
          (Components|Sphere|SetSphereRadius (Variables|Default|GetSphereComponent) (Math|Interpolation|Ease "Linear" (Math|Float|Clamp(Float) _output_get_2) (Math|Float|SelectFloat _defaultsphereradius _returnvalue_2 _newshrinkstatus) (Math|Float|SelectFloat _returnvalue_2 _defaultsphereradius _newshrinkstatus)) true)
          (Transformation|SetRelativeScale3D _staticmesh (/ (Variables|Defaults|GetDefaultRelativeMeshScale) (/ _defaultsphereradius_2 (Math|Interpolation|Ease "Linear" (Math|Float|Clamp(Float) _output_get_2) (Math|Float|SelectFloat _defaultsphereradius _returnvalue_2 _newshrinkstatus) (Math|Float|SelectFloat _returnvalue_2 _defaultsphereradius _newshrinkstatus)))))
          (Transformation|SetRelativeLocation _staticmesh (Math|Vector|MakeVector _x _y (+ _z (- _defaultsphereradius_2 (Math|Interpolation|Ease "Linear" (Math|Float|Clamp(Float) _output_get_2) (Math|Float|SelectFloat _defaultsphereradius _returnvalue_2 _newshrinkstatus) (Math|Float|SelectFloat _returnvalue_2 _defaultsphereradius _newshrinkstatus))))) false false)
          (if (>= (+ (Variables|Size|GetSizeChange_Counter) _returnvalue) 1.0)
            (goto _label_2 Close)))))))

(event EventChangeBallSize
  (params (Shrink :type Boolean))
  (bind _defaultsphereradius (Variables|Defaults|GetDefaultSphereRadius))
  (bind _staticmesh (Variables|Default|GetStaticMesh))
  (bind _defaultsphereradius_2 (Variables|Defaults|GetDefaultSphereRadius))
  (bind _defaultrelativemeshlocation (Variables|Defaults|GetDefaultRelativeMeshLocation))
  (bind _returnvalue (/ _defaultsphereradius 2.0))
  (bind (_x _y _z) (Math|Vector|BreakVector _defaultrelativemeshlocation))
  (Variables|Size|SetNewShrinkStatus Shrink)
  (Variables|Size|SetSizeChange_Counter 0.0)
  (Utilities|FlowControl|Gate true) ; enters at Open
)

(event EventBeginPlay
  (bind _staticmesh (Variables|Default|GetStaticMesh))
  (Variables|Defaults|SetDefaultSphereRadius (Class|SphereComponent|GetUnscaledSphereRadius (Variables|Default|GetSphereComponent)))
  (Variables|Defaults|SetDefaultRelativeMeshScale (Variables|/Script/Engine.SceneComponent|GetRelativeScale3D _staticmesh))
  (Variables|Defaults|SetDefaultRelativeMeshLocation (Variables|/Script/Engine.SceneComponent|GetRelativeLocation _staticmesh)))

(fn ConstructionScript)