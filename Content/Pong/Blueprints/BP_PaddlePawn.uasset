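; Player-controllable Pong paddle pawn that creates and handles the on-screen mobile interface when it belongs to the player.
; Left and right button states set a direction and open a gate on Tick to move the paddle, stopping when both or neither are pressed.
; Interface events also start, quit or toggle pause, which disables every widget except the pause widget and re-enables them on resume.
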(event Custom|PauseGame
  (Game|SetGamePaused (not (Game|IsGamePaused)))
  (if (Game|IsGamePaused)
    (Utilities|Array|Clear (Variables|Default|GetDisabledWidgets))
    (bind _foundwidgets (Widget|GetAllWidgetsOfClass "/Script/UMG.UserWidget" false))
    (for _array_element _foundwidgets
      (Utilities|Casting|CastToPauseMobileWidget _array_element
        (:CastFailed
          (Widget|SetIsEnabled _array_element false)
          (Utilities|Array|Add (Variables|Default|GetDisabledWidgets) _array_element))))
    (else
      (for _array_element_2 (Variables|Default|GetDisabledWidgets)
        (Widget|SetIsEnabled _array_element_2 true)))))

(event Custom|StateChanged_ForLeft
  (params (IsPressed :type Boolean))
  (bind _pressedright (Variables|Default|GetPressedRight))
  (bind _output_get (Variables|Default|SetPressedLeft IsPressed))
  (if _output_get
    (if (not _pressedright)
      (Variables|Default|SetCurrentDirection -1.0)
      (Utilities|FlowControl|Gate true) ; enters at Open
      (else
        (Class|PongPaddlePawn|SetVelocityZero :!label _label)
        (Utilities|FlowControl|Gate true) ; enters at Close
      ))
    (elif _pressedright
      (Variables|Default|SetCurrentDirection 1.0)
      (Utilities|FlowControl|Gate true) ; enters at Open
      (else
        (goto _label)))))

(event Custom|StateChanged_ForRight
  (params (IsPressed :type Boolean))
  (bind _pressedleft (Variables|Default|GetPressedLeft))
  (bind _output_get (Variables|Default|SetPressedRight IsPressed))
  (if _output_get
    (if (not _pressedleft)
      (Variables|Default|SetCurrentDirection 1.0)
      (Utilities|FlowControl|Gate true) ; enters at Open
      (else
        (Class|PongPaddlePawn|SetVelocityZero :!label _label)
        (Utilities|FlowControl|Gate true) ; enters at Close
      ))
    (elif _pressedleft
      (Variables|Default|SetCurrentDirection -1.0)
      (Utilities|FlowControl|Gate true) ; enters at Open
      (else
        (goto _label)))))

(event Custom|PlayGame
  (Class|PongPaddlePawn|Start))

(event Custom|ExitGame
  (Game|QuitGame 0 "Quit"))

(event EventEnablePlayButton
  (bind _mobileinterface_inst (Variables|Default|GetMobileInterface_Inst))
  (Utilities|IsValid _mobileinterface_inst
    (:Is%20Valid
      (Default|EnablePlayButton _mobileinterface_inst))))

(event EventDisablePlayButton
  (bind _mobileinterface_inst (Variables|Default|GetMobileInterface_Inst))
  (Utilities|IsValid _mobileinterface_inst
    (:Is%20Valid
      (Default|DisablePlayButton _mobileinterface_inst))))

(event EventTick
  (params (DeltaSeconds :type Float%20%28single-precision%29))
  (bind _returnvalue (Class|PongPaddlePawn|IsThisforPlayer))
  (if _returnvalue
    (Utilities|FlowControl|Gate true
      (:Exit
        (Class|PongPaddlePawn|MoveRight (Variables|Default|GetCurrentDirection))))))

(event EventBeginPlay
  (bind _returnvalue (Class|PongPaddlePawn|IsThisforPlayer))
  (if _returnvalue
    (bind _returnvalue_2 (Game|GetPlatformName))
    (switch string _returnvalue_2
      (:ANDROID
        _)
      (:IOS
        _))
    (bind _returnvalue_3 (UserInterface|CreateWidget "/Game/Pong/Widgets/MobileInterface.MobileInterface_C"))
    (bind _output_get (Variables|Default|SetMobileInterface_Inst _returnvalue_3))
    (UserInterface|Viewport|AddtoViewport _output_get 0)
    (Utilities|FlowControl|Sequence
      (:then_0
        (EventDispatchers|BindEventtoStateChangedforLeft (Variables|Default|GetMobileInterface_Inst) (delegate Custom|StateChanged_ForLeft)))
      (:then_1
        (EventDispatchers|BindEventtoStateChangedforRight (Variables|Default|GetMobileInterface_Inst) (delegate Custom|StateChanged_ForRight)))
      (:then_2
        (EventDispatchers|BindEventtoPressedPlayGame (Variables|Default|GetMobileInterface_Inst) (delegate Custom|PlayGame)))
      (:then_3
        (EventDispatchers|BindEventtoPressedExitGame (Variables|Default|GetMobileInterface_Inst) (delegate Custom|ExitGame)))
      (:then_4
        (EventDispatchers|BindEventtoPressedPauseGame (Variables|Default|GetMobileInterface_Inst) (delegate Custom|PauseGame))))))

(fn ConstructionScript)