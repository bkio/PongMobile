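; AI controller for a Pong paddle that follows the ball along the Y axis.
; Each Tick it gets all PongBall actors and, after an empty loop, uses the last one as its target.
; It moves the pawn with a swept offset at Speed times the paddle's SpeedFactor, flipping direction when IsControllerReversed is set.
; It holds still when the gap is under one frame's step, avoiding jitter.
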(event EventTick
  (params (DeltaSeconds :type Float%20%28single-precision%29))
  (bind _returnvalue (Pawn|GetControlledPawn))
  (bind _returnvalue_2 (Pawn|GetControlledPawn))
  (Utilities|IsValid _returnvalue_2
    (:Is%20Valid
      (bind _asbp_paddle_pawn (Utilities|Casting|CastToBP_PaddlePawn _returnvalue_2))
      (bind _outactors (Actor|GetAllActorsOfClass "/Script/Pong.PongBall"))
      (for _array_element _outactors
        _)
      (if (not (< (Math|Float|Absolute(Float) (- (.Y (Math|Vector|BreakVector (Transformation|GetActorLocation _array_element))) (.Y (Math|Vector|BreakVector (Transformation|GetActorLocation _returnvalue))))) (* (* (Variables|/Script/Pong.PongPaddlePawn|GetSpeedFactor _asbp_paddle_pawn) (Variables|Default|GetSpeed)) DeltaSeconds)))
        (Transformation|AddActorWorldOffset _returnvalue (Math|Vector|MakeVector 0.0 (* (* (Math|Float|Sign(Float) (- (.Y (Math|Vector|BreakVector (Transformation|GetActorLocation _array_element))) (.Y (Math|Vector|BreakVector (Transformation|GetActorLocation _returnvalue))))) (* (* (Variables|/Script/Pong.PongPaddlePawn|GetSpeedFactor _asbp_paddle_pawn) (Variables|Default|GetSpeed)) DeltaSeconds)) (Math|Float|SelectFloat -1.0 1.0 (Variables|/Script/Pong.PongPaddlePawn|GetIsControllerReversed _asbp_paddle_pawn))) 0.0) true)))))

(fn ConstructionScript)